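; BP_Collector_Rune is a spinning collectible that the third-person character picks up by overlapping it.
; Overlap increments the character's CollectionCounter, copies it into InitialFac as a float, and shows an Interfaz_coleccionable widget.
; It then destroys itself before a delayed widget removal, so that removal is unlikely to run.
; Tick rotates the root by a fixed step each frame, independent of delta time.
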(event `self.ReceiveActorBeginOverlap`
  (params (OtherActor :type "Actor Object Reference"))
  (set `self.Star` null)
  (bind _asthird_person_character (cast `/Game/ThirdPersonBP/Blueprints/ThirdPersonCharacter` OtherActor))
  (`ActorComponent.K2_DestroyComponent` (`self.estrellauwu`))
  (bind _output_get (set `/Game/ThirdPersonBP/Blueprints/ThirdPersonCharacter.CollectionCounter` (+ (`/Game/ThirdPersonBP/Blueprints/ThirdPersonCharacter.CollectionCounter` _asthird_person_character) 1) _asthird_person_character))
  (set `/Game/ThirdPersonBP/Blueprints/ThirdPersonCharacter.InitialFac` (`KismetMathLibrary.Conv_IntToDouble` _output_get) _asthird_person_character)
  (bind _returnvalue (`|CreateWidget` "/Game/Collectables/Interfaz_coleccionable.Interfaz_coleccionable_C"))
  (`UserWidget.AddToPlayerScreen` _returnvalue 0)
  (`self.K2_DestroyActor` self)
  (`KismetSystemLibrary.Delay` 10.0)
  (`Widget.RemoveFromParent` _returnvalue))

(event `self.ReceiveTick`
  (params (DeltaSeconds :type "Float (single-precision)"))
  (`SceneComponent.K2_AddLocalRotation` (`self.DefaultSceneRoot`) (struct :`Yaw` 1.0) false false))

(fn `UserConstructionScript`)