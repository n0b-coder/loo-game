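; BP_Collector is a collectable pickup that a ThirdPersonCharacter gathers by overlapping it.
; On overlap it destroys its Estrellauwu component, increments the character's CollectionCounter, shows an Interfaz_coleccionable widget on the player screen and destroys itself.
; The 10-second delayed widget removal follows DestroyActor, so it likely never runs.
; Overlaps by other actors only print a failure message.
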(event `self.ReceiveActorBeginOverlap`
  (params (OtherActor :type "Actor Object Reference"))
  (bind _asthird_person_character (cast `/Game/ThirdPersonBP/Blueprints/ThirdPersonCharacter` OtherActor)
    (:`then`
      (`ActorComponent.K2_DestroyComponent` (`self.estrellauwu`))
      (set `/Game/ThirdPersonBP/Blueprints/ThirdPersonCharacter.CollectionCounter` (+ (`/Game/ThirdPersonBP/Blueprints/ThirdPersonCharacter.CollectionCounter` _asthird_person_character) 1) _asthird_person_character)
      (bind _returnvalue (`|CreateWidget` "/Game/Collectables/Interfaz_coleccionable.Interfaz_coleccionable_C"))
      (`UserWidget.AddToPlayerScreen` _returnvalue 0)
      (`self.K2_DestroyActor` self)
      (`KismetSystemLibrary.Delay` 10.0)
      (`Widget.RemoveFromParent` _returnvalue))
    (:`CastFailed`
      (`KismetSystemLibrary.PrintString` "failed"))))

(fn `UserConstructionScript`)